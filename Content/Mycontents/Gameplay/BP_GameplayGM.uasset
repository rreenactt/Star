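; Gameplay game mode that tracks joined BP_GameplayPC controllers and refreshes the ready-room player count.
; PostLogin adds each new controller to AllPlayerControllers, then updates every WB_ReadyRoom widget found through GetAllWidgetsOfClass.
; OnLogout removes the leaving controller without refreshing the widgets.
; The OnRep for AllPlayerControllers loops over the array but does nothing.
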(event `self.K2_PostLogin`
  (params (NewPlayer :type "PlayerController Object Reference"))
  (bind _asbp_gameplay_pc (cast `/Game/Mycontents/Gameplay/BP_GameplayPC` NewPlayer))
  (`KismetArrayLibrary.Array_Add` (`self.All_PlayerControllers`) _asbp_gameplay_pc)
  (`self.UpdatePlayerUI`))

(event `UpdatePlayerUI`
  (bind _foundwidgets (`WidgetBlueprintLibrary.GetAllWidgetsOfClass` "/Game/Mycontents/Gameplay/WB_ReadyRoom.WB_ReadyRoom_C" false))
  (for _array_element _foundwidgets
    (`/Game/Mycontents/Gameplay/WB_ReadyRoom.UpdatePlayerCount` _array_element)))

(event `self.K2_OnLogout`
  (params (ExitingController :type "Controller Object Reference"))
  (bind _asbp_gameplay_pc (cast `/Game/Mycontents/Gameplay/BP_GameplayPC` ExitingController))
  (`KismetArrayLibrary.Array_RemoveItem` (`self.All_PlayerControllers`) _asbp_gameplay_pc))

(event `self.ReceiveBeginPlay`)

(fn `OnRep_All_PlayerControllers`
  (for _ (`self.All_PlayerControllers`)
    _))

(fn `UserConstructionScript`)