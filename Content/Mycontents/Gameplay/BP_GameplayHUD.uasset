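; BP_GameplayHUD is a gameplay HUD Blueprint that shows a ready-room screen with the player count.
; On BeginPlay it creates a WB_ReadyRoom widget and casts the game state to BP_GameplayGS.
; It writes the PlayerArray length over MaxPlayer into the widget's text block, then adds it to the viewport.
; The count is set only once, and a failed cast leaves the widget off screen.
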(event `self.ReceiveBeginPlay`
  (bind _returnvalue (`|CreateWidget` "/Game/Mycontents/Gameplay/WB_ReadyRoom.WB_ReadyRoom_C"))
  (bind _asbp_gameplay_gs (cast `/Game/Mycontents/Gameplay/BP_GameplayGS` (`GameplayStatics.GetGameState`)))
  (`TextBlock.SetText` (`/Game/Mycontents/Gameplay/WB_ReadyRoom.TextBlock_AmountOfPlayer` _returnvalue) (`KismetTextLibrary.Conv_StringToText` (`KismetStringLibrary.Concat_StrStr` (`KismetStringLibrary.Conv_IntToString` (`KismetArrayLibrary.Array_Length` (`GameStateBase.PlayerArray` _asbp_gameplay_gs))) "/" (`KismetStringLibrary.Conv_IntToString` (`/Game/Mycontents/Gameplay/BP_GameplayGS.MaxPlayer` _asbp_gameplay_gs)))))
  (`UserWidget.AddToViewport` _returnvalue 0))

(fn `UserConstructionScript`)