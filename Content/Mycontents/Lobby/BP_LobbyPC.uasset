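; BP_LobbyPC is the lobby player controller, handling each player's lobby UI, name and ready status.
; On BeginPlay, the local controller creates WB_LobbyUI, enables mouse input and submits the player's name.
; Name and ready-toggle events edit PlayerLobbyInfoPC and pass the controller to BP_LobbyGM's UpdatePlayerLobbyInfo, with a separate short-delay retry event.
; OnStartMatch shows the loading screen and disables input.
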(event `self.ReceiveBeginPlay`
  (`self.Setup`))

(event `TryAgainUpdatingLobbyInfo`
  (`KismetSystemLibrary.Delay` 0.1)
  (bind _asbp_lobby_gm (cast `/Game/Mycontents/Lobby/BP_LobbyGM` (`GameplayStatics.GetGameMode`)))
  (`/Game/Mycontents/Lobby/BP_LobbyGM.UpdatePlayerLobbyInfo` _asbp_lobby_gm self))

(event `SetPlayerNameOnServer`
  (params (PlayerName :type Text))
  (setmembers `/Game/Mycontents/Lobby/S_PlayerLobbyInfo` :`StructRef` (`self.PlayerLobbyInfoPC`) :`PlayerName` PlayerName)
  (bind _asbp_lobby_gm (cast `/Game/Mycontents/Lobby/BP_LobbyGM` (`GameplayStatics.GetGameMode`)))
  (`/Game/Mycontents/Lobby/BP_LobbyGM.UpdatePlayerLobbyInfo` _asbp_lobby_gm self))

(event `ToggleReadyStatusOnServer`
  (bind _playerlobbyinfopc (`self.PlayerLobbyInfoPC`))
  (setmembers `/Game/Mycontents/Lobby/S_PlayerLobbyInfo` :`StructRef` _playerlobbyinfopc :`bReady` (not (`.bReady_8_404E476E4926A76699068EB8DAF5149D` (break `/Game/Mycontents/Lobby/S_PlayerLobbyInfo` _playerlobbyinfopc))))
  (bind _asbp_lobby_gm (cast `/Game/Mycontents/Lobby/BP_LobbyGM` (`GameplayStatics.GetGameMode`)))
  (`/Game/Mycontents/Lobby/BP_LobbyGM.UpdatePlayerLobbyInfo` _asbp_lobby_gm self))

(event `OnStartMatch`
  (`/Game/Mycontents/Lobby/WB_LobbyUI.ShowLoadingScreen` (`self.LobbyUI_Ref`))
  (`self.DisableInput` self))

(fn `Setup`
  (if (`self.IsLocalPlayerController`)
    (set `self.bShowMouseCursor` true)
    (`WidgetBlueprintLibrary.SetInputMode_GameAndUIEx` self null "DoNotLock" false)
    (bind _returnvalue (`|CreateWidget` "/Game/Mycontents/Lobby/WB_LobbyUI.WB_LobbyUI_C"))
    (bind _output_get (set `self.LobbyUI_Ref` _returnvalue))
    (`UserWidget.AddToViewport` _output_get 0)
    (`self.SetPlayerNameOnServer` (`KismetTextLibrary.Conv_StringToText` (`AdvancedSessionsLibrary.GetPlayerName` self)))))

(fn `UserConstructionScript`)