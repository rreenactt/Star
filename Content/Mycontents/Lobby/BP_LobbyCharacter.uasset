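; Lobby character that shows a player's skeletal mesh and an info widget in the game lobby.
; UpdatePlayerLobbyInfo sets PlayerLobbyInfo, whose RepNotify passes it to the WB_PlayerLobbyInfo widget and makes the LobbyInfo component visible.
; If the widget is not yet valid, the RepNotify retries itself on a short timer.
; MC_-prefixed events swap the character mesh and play a non-looping animation on it.
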(event `MC_SetPlayerMesh`
  (params (NewMesh :type "SkeletalMesh Object Reference"))
  (`SkeletalMeshComponent.SetSkeletalMeshAsset` (`self.CharacterMesh`) NewMesh))

(event `MC_PlayerMeshAnim`
  (`SkeletalMeshComponent.PlayAnimation` (`self.CharacterMesh`) null false))

(fn `OnRep_PlayerLobbyInfo`
  (bind _returnvalue (`WidgetComponent.GetWidget` (`self.LobbyInfo`)))
  (`/Engine/EditorBlueprintResources/StandardMacros.IsValid` _returnvalue
    (:`Is Valid`
      (bind _aswb_player_lobby_info (cast `/Game/Mycontents/Lobby/WB_PlayerLobbyInfo` _returnvalue))
      (`/Game/Mycontents/Lobby/WB_PlayerLobbyInfo.Update` _aswb_player_lobby_info (`self.PlayerLobbyInfo`))
      (`SceneComponent.SetVisibility` (`self.LobbyInfo`) true false))
    (:`Is Not Valid`
      (`KismetSystemLibrary.K2_SetTimer` null "OnRep_PlayerLobbyInfo" 0.1))))

(fn `UpdatePlayerLobbyInfo`
  (params (PlayerLobbyInfo :type "/Game/Mycontents/Lobby/S_PlayerLobbyInfo Structure"))
  (set `self.PlayerLobbyInfo` PlayerLobbyInfo))

(fn `UserConstructionScript`)